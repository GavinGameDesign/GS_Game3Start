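; BP_NodeManager is a manager that grows an endless chain of node actors through the level for as long as it runs.
; BeginPlay spawns the first node at the manager's location, then SpawnNewNode re-calls itself after a two-second Delay with no stop condition.
; Each new BP_Node appears at a random point in a box around the last one, gets a running index, and links both ways as a doubly linked list.
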(event Custom|SpawnNewNode
  (bind _nodeindex (Variables|Default|GetNodeIndex))
  (bind _returnvalue (Game|SpawnActorfromClass "/Game/Blueprints/VisualizeNodes/BP_Node.BP_Node_C" (Math|Transform|MakeTransform (Math|Random|RandomPointinBoundingBox (Transformation|GetActorLocation (Variables|Default|GetLastNode)) "500.000000,500.000000,500.000000") "0, 0, 0" "1.000000,1.000000,1.000000") "Undefined" "MultiplyWithRoot" 0 0))
  (Variables|/Game/Blueprints/VisualizeNodes/BP_Node.BP_Node_C|SetPrevNode _returnvalue (Variables|Default|GetLastNode))
  (Variables|/Game/Blueprints/VisualizeNodes/BP_Node.BP_Node_C|SetIndex _returnvalue _nodeindex)
  (Math|Integer|IncrementInt _nodeindex
    (:%20%20
      (Variables|/Game/Blueprints/VisualizeNodes/BP_Node.BP_Node_C|SetNextNode (Variables|Default|GetLastNode) _returnvalue)
      (Variables|Default|SetLastNode _returnvalue)
      (Utilities|FlowControl|Delay 2.0)
      (CallFunction|SpawnNewNode))))

(event EventBeginPlay
  (bind _returnvalue (Game|SpawnActorfromClass "/Game/Blueprints/VisualizeNodes/BP_Node.BP_Node_C" (Math|Transform|MakeTransform (Transformation|GetActorLocation) "0, 0, 0" "1.000000,1.000000,1.000000") "Undefined" "MultiplyWithRoot" 0 0))
  (Variables|Default|SetLastNode _returnvalue)
  (bind _output_get (Variables|/Game/Blueprints/VisualizeNodes/BP_Node.BP_Node_C|SetIndex _returnvalue (Variables|Default|GetNodeIndex)))
  (Variables|Default|SetNodeIndex (+ _output_get 1))
  (CallFunction|SpawnNewNode))

(fn ConstructionScript)