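; Debug visualizer actor that demonstrates HSV color interpolation with debug spheres.
; On BeginPlay it draws a vertical column of ten spheres above itself, shading from cyan toward red as Step drives height and lerp alpha.
; It repeats after each sphere lifetime without resetting Step, so later batches climb higher with alpha beyond one.
; An unconnected timeline holds a single large sphere animated from blue to red.
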(event EventBeginPlay
  (bind _returnvalue (Transformation|GetActorLocation))
  (for _index (range 0 9) :!label _label
    (Rendering|Debug|DrawDebugSphere (Math|Vector|MakeVector (.x _returnvalue) (.y _returnvalue) (+ (.z _returnvalue) (* (Variables|Default|GetStep) 5e+02))) 3e+01 30 (Class|KismetMathLibrary|LinearColorLerpUsingHSV "(R=0.000000,G=1.000000,B=1.000000,A=1.000000)" "(R=1.000000,G=0.000000,B=0.000000,A=1.000000)" (Variables|Default|GetStep)) 1e+01 2.0)
    (Variables|Default|SetStep (+ (Variables|Default|GetStep) 0.1)))
  (Utilities|FlowControl|Delay 1e+01)
  (goto _label))

(fn ConstructionScript)