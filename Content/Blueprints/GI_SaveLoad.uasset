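; GI_SaveLoad handles saving the player's state to a save slot, with loading only stubbed out as a debug print.
; SaveGame loads the existing SG_Coding2 object from the slot or creates one if none exists.
; It copies the third-person character's stamina, capsule world transform and sprint and shoot permissions into that object, then writes it back to the slot.
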(event Custom|Save%20Game
  (Development|PrintString "Startubg Save Game")
  (bind _returnvalue (SaveGame|DoesSaveGameExist (Variables|Default|GetSlot%20Name)))
  (if _returnvalue
    (bind _returnvalue_2 (SaveGame|LoadGamefromSlot (Variables|Default|GetSlot%20Name)))
    (Variables|Default|SetSaverSubclass _returnvalue_2)
    (else
      (bind _returnvalue_3 (SaveGame|CreateSaveGameObject "/Game/Blueprints/SG_Coding2.SG_Coding2_C"))
      (Variables|Default|SetSaverSubclass _returnvalue_3)))
  (bind _assg_coding_2 (Utilities|Casting|CastToSG_Coding2 (Variables|Default|GetSaverSubclass)))
  (bind _asbp_third_person_character (Utilities|Casting|CastToBP_ThirdPersonCharacter (Game|GetPlayerCharacter 0)))
  (Variables|/Game/Blueprints/SG_Coding2.SG_Coding2_C|SetPlayerStamina _assg_coding_2 (Variables|/Game/ThirdPerson/Blueprints/BP_ThirdPersonCharacter.BP_ThirdPersonCharacter_C|GetStamina _asbp_third_person_character))
  (Variables|/Game/Blueprints/SG_Coding2.SG_Coding2_C|SetPlayerTransform _assg_coding_2 (Transformation|GetWorldTransform (Variables|/Script/Engine.Character|GetCapsuleComponent _asbp_third_person_character)))
  (Variables|/Game/Blueprints/SG_Coding2.SG_Coding2_C|SetPlayerCanSprint _assg_coding_2 (Variables|/Game/ThirdPerson/Blueprints/BP_ThirdPersonCharacter.BP_ThirdPersonCharacter_C|GetCanSprint _asbp_third_person_character))
  (Variables|/Game/Blueprints/SG_Coding2.SG_Coding2_C|SetPlayerCanShoot _assg_coding_2 (Variables|/Game/ThirdPerson/Blueprints/BP_ThirdPersonCharacter.BP_ThirdPersonCharacter_C|GetCanShoot _asbp_third_person_character))
  (SaveGame|SaveGametoSlot _assg_coding_2 (Variables|Default|GetSlot%20Name))
  (Development|PrintString "SAVED"))

(event Custom|Load%20Game
  (Development|PrintString "Starting Load Game"))