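; Debug prototype actor that simulates and visualizes projectile bullet drop from an Arrow component.
; A custom event steps the path in segments, line tracing and drawing each, applying gravity to velocity and stopping on a hit.
; A disconnected repeating chain pairs it with the engine's projectile path prediction, but BeginPlay is empty, so it never runs.
; A separate PredictProjectile function computes straight-line segments by index without gravity.
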(event Custom|ReallyCoolBulletDropCalculator
  (bind _maxsimtime (Variables|Default|GetMaxSimTime))
  (Variables|Default|SetEnd (+ (Variables|Default|GetStartLocation) (/ (Variables|Default|GetVelocity) (Math|Vector|MakeVector (Variables|Default|GetSimFrequency) 1.0 1.0))))
  (Utilities|FlowControl|ForLoopwithBreak 1 (Math|Float|Truncate (Variables|Default|GetSimFrequency))
    (:LoopBody
      (Rendering|Debug|DrawDebugLine (Variables|Default|GetStartLocation) (Variables|Default|GetEnd) "(R=0.000000,G=0.454646,B=1.000000,A=1.000000)" _maxsimtime 0.0)
      (Rendering|Debug|DrawDebugSphere (Variables|Default|GetEnd) 5.0 12 "(R=0.000000,G=0.456411,B=1.000000,A=1.000000)" _maxsimtime)
      (bind _returnvalue (Class|KismetSystemLibrary|LineTraceSinglebyProfile (Variables|Default|GetStartLocation) (Variables|Default|GetEnd) "BlockAll" false 0 "None" true))
      (if _returnvalue
        (Development|PrintString "HIT" true true "(R=1.000000,G=0.000000,B=0.006161,A=1.000000)" 5.0)
        (CallFunction|Break)
        (else
          (Variables|Default|SetStartLocation (Variables|Default|GetEnd))
          (Variables|Default|SetVelocity (+ (Variables|Default|GetVelocity) (Math|Vector|MakeVector 0.0 0.0 (/ -9.8e+02 (Math|Float|Square (Variables|Default|GetSimFrequency))))))
          (Variables|Default|SetEnd (+ (Variables|Default|GetStartLocation) (/ (Variables|Default|GetVelocity) (Math|Vector|MakeVector (Variables|Default|GetSimFrequency) 1.0 1.0)))))))
    (:Completed
      (Variables|Default|SetStartLocation (Transformation|GetWorldLocation (Variables|Default|GetArrow)))
      (Variables|Default|SetVelocity (Variables|Default|GetStartingVelocity)))))

(event Custom|Break
  (bind _maxsimtime (Variables|Default|GetMaxSimTime))
  (Utilities|FlowControl|ForLoopwithBreak 1 (Math|Float|Truncate (Variables|Default|GetSimFrequency))) ; enters at Break
)

(event EventBeginPlay)

(fn ConstructionScript)

(fn PredictProjectile
  (params (Index :type Integer))
  (bind _simfrequency (Variables|Default|GetSimFrequency))
  (bind _velocity (Variables|Default|GetVelocity))
  (bind _returnvalue (/ _velocity _simfrequency))
  (bind _output_get (Variables|Default|SetCurrentPosition (- (+ (* _returnvalue Index) (Variables|Default|GetStartLocation)) (Math|Vector|MakeVector 0.0 0.0 0.0))))
  (return _output_get (+ _output_get _returnvalue)))