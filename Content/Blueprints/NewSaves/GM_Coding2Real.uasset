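; Game mode that handles per-level save games, using the current level name as the save slot.
; On BeginPlay it loads or creates an SG_LevelSaveReal, restores collected coins and moves the player capsule to the saved transform unless its location is zero.
; Checkpoint stores a player transform and saves, while FinishedLevel clears it and saves.
; DeleteGame removes the slot and reopens the level.
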(event Custom|Save%20Game
  (bind _returnvalue (Game|GetCurrentLevelName true))
  (bind _returnvalue_2 (SaveGame|SaveGametoSlot (Variables|Default|GetLevelSave) _returnvalue))
  (if _returnvalue_2
    (Development|PrintString "Saved level" true true "(R=0.000000,G=1.000000,B=0.000000,A=1.000000)" 5.0)
    (else
      (Development|PrintString "Could not save level" true true "(R=1.000000,G=0.000000,B=0.007327,A=1.000000)" 5.0))))

(event Custom|Delete%20Game
  (bind _returnvalue (Game|GetCurrentLevelName true))
  (bind _returnvalue_2 (SaveGame|DeleteGameinSlot _returnvalue))
  (if _returnvalue_2
    (Development|PrintString "Deleted Save" true true "(R=0.000000,G=1.000000,B=0.000000,A=1.000000)" 5.0)
    (Game|OpenLevel(byName) (Utilities|String|StringToName _returnvalue))
    (else
      (Development|PrintString "No Save To Delete" true true "(R=1.000000,G=0.000000,B=0.000000,A=1.000000)" 5.0))))

(event EventBeginPlay
  (bind _returnvalue (Game|GetCurrentLevelName true))
  (bind _returnvalue_2 (SaveGame|DoesSaveGameExist _returnvalue))
  (if _returnvalue_2
    (bind _returnvalue_3 (SaveGame|LoadGamefromSlot _returnvalue))
    (bind _assg_level_save_real (Utilities|Casting|CastToSG_LevelSaveReal _returnvalue_3))
    (bind _output_get (Variables|Default|SetLevelSave _assg_level_save_real))
    (Default|LoadCollectedCoins _output_get)
    (if (not (Class|KismetMathLibrary|EqualExactlyVectorVector (.location (Variables|/Game/Blueprints/NewSaves/SG_LevelSaveReal.SG_LevelSaveReal_C|GetPlayerTransform (Variables|Default|GetLevelSave))) "0, 0, 0"))
      (Transformation|SetWorldTransform (Variables|/Script/Engine.Character|GetCapsuleComponent (Game|GetPlayerCharacter 0)) (Variables|/Game/Blueprints/NewSaves/SG_LevelSaveReal.SG_LevelSaveReal_C|GetPlayerTransform (Variables|Default|GetLevelSave)) false false))
    (else
      (bind _returnvalue_4 (SaveGame|CreateSaveGameObject "/Game/Blueprints/NewSaves/SG_LevelSaveReal.SG_LevelSaveReal_C"))
      (Variables|Default|SetLevelSave _returnvalue_4))))

(fn ConstructionScript)

(fn Checkpoint
  (params (PlayerTransform :type Transform))
  (Variables|/Game/Blueprints/NewSaves/SG_LevelSaveReal.SG_LevelSaveReal_C|SetPlayerTransform (Variables|Default|GetLevelSave) PlayerTransform)
  (CallFunction|SaveGame))

(fn FinishedLevel
  (Variables|/Game/Blueprints/NewSaves/SG_LevelSaveReal.SG_LevelSaveReal_C|SetPlayerTransform (Variables|Default|GetLevelSave) "")
  (CallFunction|SaveGame))