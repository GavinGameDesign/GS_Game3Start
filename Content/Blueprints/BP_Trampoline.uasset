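; Trampoline actor that launches the third-person character upward shortly after overlap and can be carried and repositioned.
; Stationary instances remove their handles and grab-range box and turn parts red.
; While the player is in range, GrabTrampoline alternately attaches it to and detaches it from the character.
; The first grab registers it in the game mode's LevelSave, and each drop inserts its transform there at the stored index.
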(event OnComponentBeginOverlap(Box)
  (params (OverlappedComponent :type Primitive%20Component%20Object%20Reference) (OtherActor :type Actor%20Object%20Reference) (OtherComp :type Primitive%20Component%20Object%20Reference) (OtherBodyIndex :type Integer) (bFromSweep :type Boolean) (SweepResult :type Hit%20Result%20Structure%20%28by%20ref%29))
  (bind _asbp_third_person_character (Utilities|Casting|CastToBP_ThirdPersonCharacter OtherActor))
  (CallFunction|Jump _asbp_third_person_character))

(event OnComponentBeginOverlap(Box1)
  (params (OverlappedComponent :type Primitive%20Component%20Object%20Reference) (OtherActor :type Actor%20Object%20Reference) (OtherComp :type Primitive%20Component%20Object%20Reference) (OtherBodyIndex :type Integer) (bFromSweep :type Boolean) (SweepResult :type Hit%20Result%20Structure%20%28by%20ref%29))
  (Utilities|Casting|CastToBP_ThirdPersonCharacter OtherActor)
  (Variables|Default|SetInRange true))

(event OnComponentEndOverlap(Box1)
  (params (OverlappedComponent :type Primitive%20Component%20Object%20Reference) (OtherActor :type Actor%20Object%20Reference) (OtherComp :type Primitive%20Component%20Object%20Reference) (OtherBodyIndex :type Integer))
  (Utilities|Casting|CastToBP_ThirdPersonCharacter OtherActor)
  (Variables|Default|SetInRange false))

(event Custom|Jump
  (params (JumpingPlayer :type BP%20Third%20Person%20Character%20Object%20Reference))
  (Utilities|FlowControl|Delay 0.1)
  (Character|LaunchCharacter JumpingPlayer "0.000000,0.000000,4000.000000" false false))

(event Custom|GrabTrampoline
  (if (Variables|Default|GetInRange)
    (if (Variables|Default|GetHasBeenMoved)
      _
      (else
        (bind _asgm_coding_2real (Utilities|Casting|CastToGM_Coding2Real (Game|GetGameMode)))
        (bind _returnvalue (Utilities|Array|AddUnique (Variables|/Game/Blueprints/NewSaves/SG_LevelSaveReal.SG_LevelSaveReal_C|GetTrampolines (Variables|/Game/Blueprints/NewSaves/GM_Coding2Real.GM_Coding2Real_C|GetLevelSave _asgm_coding_2real)) self))
        (Variables|Default|SetTrampolineIndex _returnvalue)
        (Variables|Default|SetHasBeenMoved true)))
    (Utilities|FlowControl|FlipFlop
      (:A
        (Transformation|AttachActorToActor (Variables|Default|GetThirdPersonCharacter) "None" "KeepWorld" "KeepWorld" "KeepWorld" true))
      (:B
        (Transformation|DetachFromActor "KeepWorld" "KeepWorld" "KeepWorld")
        (Utilities|Array|Insert (Variables|/Game/Blueprints/NewSaves/SG_LevelSaveReal.SG_LevelSaveReal_C|GetTrampolineTransform (Variables|/Game/Blueprints/NewSaves/GM_Coding2Real.GM_Coding2Real_C|GetLevelSave _asgm_coding_2real)) (Transformation|GetWorldTransform (Variables|Default|GetDefaultSceneRoot)) (Variables|Default|GetTrampolineIndex))))))

(event Custom|RemoveHandles
  (Components|DestroyComponent (Variables|Default|GetCylinder))
  (Rendering|Material|SetMaterial (Variables|Default|GetCube3) 0 "/Game/Materials/MI_FlatRed.MI_FlatRed"))

(event EventBeginPlay
  (bind _returnvalue (Actor|GetActorOfClass "/Game/ThirdPerson/Blueprints/BP_ThirdPersonCharacter.BP_ThirdPersonCharacter_C"))
  (Variables|Default|SetThirdPersonCharacter _returnvalue)
  (if (Variables|Default|GetIsStationary)
    (CallFunction|RemoveHandles)))

(fn ConstructionScript)