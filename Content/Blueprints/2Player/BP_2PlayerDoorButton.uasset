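; BP_2PlayerDoorButton is a button, kept in the two-player folder, that drives a linked door when a third-person character stands on it.
; Sphere1 overlap begin and end events filter for BP_ThirdPersonCharacter, then switch on ButtonNumber to call the matching Activate or Deactivate function on the Door reference.
; Each instance acts as button 0 or button 1, and the door receives their states separately.
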(event OnComponentBeginOverlap(Sphere1)
  (params (OverlappedComponent :type Primitive%20Component%20Object%20Reference) (OtherActor :type Actor%20Object%20Reference) (OtherComp :type Primitive%20Component%20Object%20Reference) (OtherBodyIndex :type Integer) (bFromSweep :type Boolean) (SweepResult :type Hit%20Result%20Structure%20%28by%20ref%29))
  (bind _door (Variables|Default|GetDoor))
  (Utilities|Casting|CastToBP_ThirdPersonCharacter OtherActor)
  (switch int (Variables|Default|GetButtonNumber)
    (:0
      (Default|ActivateButton0 _door))
    (:1
      (Default|ActivateButton1 _door))))

(event OnComponentEndOverlap(Sphere1)
  (params (OverlappedComponent :type Primitive%20Component%20Object%20Reference) (OtherActor :type Actor%20Object%20Reference) (OtherComp :type Primitive%20Component%20Object%20Reference) (OtherBodyIndex :type Integer))
  (bind _door (Variables|Default|GetDoor))
  (Utilities|Casting|CastToBP_ThirdPersonCharacter OtherActor)
  (switch int (Variables|Default|GetButtonNumber)
    (:0
      (Default|DeactivateButton0 _door))
    (:1
      (Default|DeactivateButton1 _door))))

(fn ConstructionScript)