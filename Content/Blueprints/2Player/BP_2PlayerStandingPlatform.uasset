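; Co-op moving platform that travels from Start to End only while two third-person characters stand on it, reversing when either steps off.
; Box overlaps track both players and drive a Timeline that lerps MovePoint, with play rate set from MoveTime.
; Each Timeline update triggers camera shake and force feedback for players on top.
; BeginPlay randomly keeps one of three floating island meshes and destroys the others.
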(event OnComponentBeginOverlap(Box)
  (params (OverlappedComponent :type Primitive%20Component%20Object%20Reference) (OtherActor :type Actor%20Object%20Reference) (OtherComp :type Primitive%20Component%20Object%20Reference) (OtherBodyIndex :type Integer) (bFromSweep :type Boolean) (SweepResult :type Hit%20Result%20Structure%20%28by%20ref%29))
  (bind _asbp_third_person_character (Utilities|Casting|CastToBP_ThirdPersonCharacter OtherActor))
  (Utilities|IsValid (Variables|Default|GetFirstPlayerOnTop)
    (:Is%20Valid
      (Variables|Default|SetSecondPlayerOnTop _asbp_third_person_character))
    (:Is%20Not%20Valid
      (Variables|Default|SetFirstPlayerOnTop _asbp_third_person_character)))
  (CallFunction|CheckforStart))

(event OnComponentEndOverlap(Box)
  (params (OverlappedComponent :type Primitive%20Component%20Object%20Reference) (OtherActor :type Actor%20Object%20Reference) (OtherComp :type Primitive%20Component%20Object%20Reference) (OtherBodyIndex :type Integer))
  (bind _asbp_third_person_character (Utilities|Casting|CastToBP_ThirdPersonCharacter OtherActor))
  (if (== _asbp_third_person_character (Variables|Default|GetFirstPlayerOnTop))
    (Variables|Default|SetFirstPlayerOnTop 0)
    (else
      (Variables|Default|SetSecondPlayerOnTop 0)))
  (CallFunction|CheckforStop))

(event Custom|CheckForStart
  (Utilities|IsValid (Variables|Default|GetFirstPlayerOnTop)
    (:Is%20Valid
      (Utilities|IsValid (Variables|Default|GetSecondPlayerOnTop)
        (:Is%20Valid
          (bind _newtrack_0 (Timeline|Timeline Play)
            (:Update
              (Transformation|SetRelativeLocation (Variables|Default|GetMovePoint) (Math|Vector|Lerp(Vector) (Variables|/Script/Engine.SceneComponent|GetRelativeLocation (Variables|Default|GetStart)) (Variables|/Script/Engine.SceneComponent|GetRelativeLocation (Variables|Default|GetEnd)) _newtrack_0) false false)
              (CallFunction|Shake))))))))

(event Custom|CheckForStop
  (Utilities|IsValid (Variables|Default|GetFirstPlayerOnTop)
    (:Is%20Valid
      (Utilities|IsValid (Variables|Default|GetSecondPlayerOnTop)
        (:Is%20Not%20Valid
          (bind _newtrack_0 (Timeline|Timeline Reverse)
            (:Update
              (Transformation|SetRelativeLocation (Variables|Default|GetMovePoint) (Math|Vector|Lerp(Vector) (Variables|/Script/Engine.SceneComponent|GetRelativeLocation (Variables|Default|GetStart)) (Variables|/Script/Engine.SceneComponent|GetRelativeLocation (Variables|Default|GetEnd)) _newtrack_0) false false)
              (CallFunction|Shake))))))
    (:Is%20Not%20Valid
      (Timeline|Timeline Reverse))))

(event Custom|Shake
  (bind _secondplayerontop (Variables|Default|GetSecondPlayerOnTop))
  (bind _firstplayerontop (Variables|Default|GetFirstPlayerOnTop))
  (bind _returnvalue (Pawn|GetLocalViewingPlayerController _secondplayerontop))
  (bind _returnvalue_2 (Pawn|GetLocalViewingPlayerController _firstplayerontop))
  (Utilities|IsValid _firstplayerontop
    (:Is%20Valid
      (Game|Feedback|ClientStartCameraShake _returnvalue_2 "/Game/Blueprints/2Player/CS_PlatformShake.CS_PlatformShake_C" 1.0 "CameraLocal" "0, 0, 0")
      (Game|Feedback|ClientPlayForceFeedback _returnvalue_2 "/Game/Input/ForceFeedback/FFE_Quick.FFE_Quick" "None" false false false))
    (:Is%20Not%20Valid
      _))
  (Utilities|IsValid _secondplayerontop
    (:Is%20Valid
      (Game|Feedback|ClientStartCameraShake _returnvalue "/Game/Blueprints/2Player/CS_PlatformShake.CS_PlatformShake_C" 1.0 "CameraLocal" "0, 0, 0")
      (Game|Feedback|ClientPlayForceFeedback _returnvalue "/Game/Input/ForceFeedback/FFE_Quick.FFE_Quick" "None" false false false))))

(event Custom|StopShake)

(event EventBeginPlay
  (bind _sm_floatingsquareislanda (Variables|Default|GetSM_FloatingSquareIslandA))
  (Utilities|FlowControl|Sequence
    (:then_0
      (Components|Timeline|SetPlayRate (Variables|Default|GetTimeline) (/ 1.0 (Variables|Default|GetMoveTime))))
    (:then_1
      (switch int (Math|Random|RandomIntegerinRange 0 2)
        (:0
          (Components|DestroyComponent (Variables|Default|GetSM_FloatingSquareIslandB)))
        (:1
          (Components|DestroyComponent _sm_floatingsquareislanda))
        (:2
          (Components|DestroyComponent _sm_floatingsquareislanda))))))

(fn ConstructionScript)