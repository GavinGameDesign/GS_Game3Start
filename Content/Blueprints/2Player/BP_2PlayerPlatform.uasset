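; Two-player moving platform that travels between Start and End points while at least one player stands on a button.
; Button events track up to two players, playing a MoveTime-scaled Timeline that lerps MovePoint and reversing it once both slots empty.
; BeginPlay randomly keeps one of three floating island meshes.
; A Box overlap tracks the riding character, who gets camera shake and force feedback as the Timeline updates.
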(event OnComponentBeginOverlap(Box)
  (params (OverlappedComponent :type Primitive%20Component%20Object%20Reference) (OtherActor :type Actor%20Object%20Reference) (OtherComp :type Primitive%20Component%20Object%20Reference) (OtherBodyIndex :type Integer) (bFromSweep :type Boolean) (SweepResult :type Hit%20Result%20Structure%20%28by%20ref%29))
  (bind _asbp_third_person_character (Utilities|Casting|CastToBP_ThirdPersonCharacter OtherActor))
  (Variables|Default|SetPlayerOnTop _asbp_third_person_character))

(event OnComponentEndOverlap(Box)
  (params (OverlappedComponent :type Primitive%20Component%20Object%20Reference) (OtherActor :type Actor%20Object%20Reference) (OtherComp :type Primitive%20Component%20Object%20Reference) (OtherBodyIndex :type Integer))
  (Utilities|Casting|CastToBP_ThirdPersonCharacter OtherActor)
  (CallFunction|StopShake)
  (Utilities|FlowControl|Delay 0.2)
  (Variables|Default|SetPlayerOnTop 0))

(event Custom|StartMoving
  (bind _newtrack_0 (Timeline|Timeline Play)
    (:Update
      (Transformation|SetRelativeLocation (Variables|Default|GetMovePoint) (Math|Vector|Lerp(Vector) (Variables|/Script/Engine.SceneComponent|GetRelativeLocation (Variables|Default|GetStart)) (Variables|/Script/Engine.SceneComponent|GetRelativeLocation (Variables|Default|GetEnd)) _newtrack_0) false false)
      (CallFunction|Shake))))

(event Custom|StopMoving
  (Utilities|IsValid (Variables|Default|GetPlayerOnButton1)
    (:Is%20Not%20Valid
      (Utilities|IsValid (Variables|Default|GetPlayerOnButton2)
        (:Is%20Not%20Valid
          (bind _newtrack_0 (Timeline|Timeline Reverse)
            (:Update
              (Transformation|SetRelativeLocation (Variables|Default|GetMovePoint) (Math|Vector|Lerp(Vector) (Variables|/Script/Engine.SceneComponent|GetRelativeLocation (Variables|Default|GetStart)) (Variables|/Script/Engine.SceneComponent|GetRelativeLocation (Variables|Default|GetEnd)) _newtrack_0) false false)
              (CallFunction|Shake))))))))

(event Custom|Shake
  (bind _playerontop (Variables|Default|GetPlayerOnTop))
  (bind _returnvalue (Pawn|GetLocalViewingPlayerController _playerontop))
  (Utilities|IsValid _playerontop
    (:Is%20Valid
      (Game|Feedback|ClientStartCameraShake _returnvalue "/Game/Blueprints/2Player/CS_PlatformShake.CS_PlatformShake_C" 1.0 "CameraLocal" "0, 0, 0")
      (Game|Feedback|ClientPlayForceFeedback _returnvalue "/Game/Input/ForceFeedback/FFE_Quick.FFE_Quick" "None" false false false))))

(event Custom|StopShake
  (bind _playerontop (Variables|Default|GetPlayerOnTop))
  (Utilities|IsValid _playerontop
    (:Is%20Valid
      (Game|Feedback|ClientStopCameraShake (Pawn|GetLocalViewingPlayerController _playerontop) "/Game/Blueprints/2Player/CS_PlatformShake.CS_PlatformShake_C" true))))

(event Custom|SteppedOnButton
  (params (Player :type BP%20Third%20Person%20Character%20Object%20Reference))
  (Utilities|IsValid (Variables|Default|GetPlayerOnButton1)
    (:Is%20Valid
      (Variables|Default|SetPlayerOnButton2 Player))
    (:Is%20Not%20Valid
      (Variables|Default|SetPlayerOnButton1 Player)))
  (CallFunction|StartMoving))

(event Custom|SteppedOffButton
  (params (Player :type BP%20Third%20Person%20Character%20Object%20Reference))
  (if (== Player (Variables|Default|GetPlayerOnButton1))
    (Variables|Default|SetPlayerOnButton1 0)
    (else
      (Variables|Default|SetPlayerOnButton2 0)))
  (CallFunction|StopMoving))

(event EventBeginPlay
  (bind _sm_floatingsquareislanda (Variables|Default|GetSM_FloatingSquareIslandA))
  (Utilities|FlowControl|Sequence
    (:then_0
      (Components|Timeline|SetPlayRate (Variables|Default|GetTimeline) (/ 1.0 (Variables|Default|GetMoveTime))))
    (:then_1
      (switch int (Math|Random|RandomIntegerinRange 0 2)
        (:0
          (Components|DestroyComponent (Variables|Default|GetSM_FloatingSquareIslandB)))
        (:1
          (Components|DestroyComponent _sm_floatingsquareislanda))
        (:2
          (Components|DestroyComponent _sm_floatingsquareislanda))))))

(fn ConstructionScript)