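; Two-player co-op door that opens once both of its buttons are active at the same time.
; Button events set two flags, and each activation checks them while the door is still closed.
; Opening lowers the cliff mesh on a timeline with camera shake and force feedback for both players, and releasing a button does not re-close it.
; QuietOpen is a separate timeline-driven lowering without feedback, marking the door open when finished.
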(event Custom|OpenDoor
  (bind _returnvalue (Game|GetPlayerController 0))
  (Variables|Default|SetClosed false)
  (Game|Feedback|ClientStartCameraShake _returnvalue "/Game/Blueprints/2Player/CS_DoorShake.CS_DoorShake_C" 1.0 "World" "0, 0, 0")
  (Game|Feedback|ClientPlayForceFeedback _returnvalue "/Game/Input/ForceFeedback/FFE_DoorShake.FFE_DoorShake" "None" false false false)
  (bind _newtrack_0 (Timeline|Timeline Play)
    (:Update
      (Transformation|SetRelativeLocation (Variables|Default|GetSM_CliffC) (Math|Vector|Lerp(Vector) "0, 0, 0" "0.000000,0.000000,-430.000000" _newtrack_0) false false))))

(event Custom|QuietOpen
  (bind _newtrack_0 (Timeline|Timeline_0 Play)
    (:Update
      (Transformation|SetRelativeLocation (Variables|Default|GetSM_CliffC) (Math|Vector|Lerp(Vector) "0.000000,0.000000,150.000000" "0.000000,0.000000,-130.000000" _newtrack_0) false false))
    (:Finished
      (Variables|Default|SetClosed false))))

(event Custom|ActivateButton0
  (Variables|Default|SetButton0Active true)
  (CallFunction|CheckButtons))

(event Custom|ActivateButton1
  (Variables|Default|SetButton1Active true)
  (CallFunction|CheckButtons))

(event Custom|CheckButtons
  (if (Variables|Default|GetClosed)
    (if (Variables|Default|GetButton0Active)
      (if (Variables|Default|GetButton1Active)
        (CallFunction|OpenDoor)))))

(event Custom|DeactivateButton1
  (Variables|Default|SetButton1Active false))

(event Custom|DeactivateButton0
  (Variables|Default|SetButton0Active false))

(fn ConstructionScript)