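; Door actor that slides down to open, showing the moment through a camera cut.
; OpenDoor, if still closed, records itself in the game mode's LevelSave, blends the player's view to the door, plays the slide timeline, then after a pause blends back to the supplied view target.
; QuietOpen runs its own timeline for the same slide without camera or save steps; both paths clear Closed when finished.
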(event Custom|OpenDoor
  (params (NewViewTarget :type Actor%20Object%20Reference))
  (if (Variables|Default|GetClosed)
    (bind _asgm_coding_2real (Utilities|Casting|CastToGM_Coding2Real (Game|GetGameMode)))
    (Utilities|Array|AddUnique (Variables|/Game/Blueprints/NewSaves/SG_LevelSaveReal.SG_LevelSaveReal_C|GetOpenedDoors (Variables|/Game/Blueprints/NewSaves/GM_Coding2Real.GM_Coding2Real_C|GetLevelSave _asgm_coding_2real)) self)
    (Game|Player|SetViewTargetwithBlend (Game|GetPlayerController 0) self (Variables|Default|GetBlend%20Time) "VTBlend_Cubic" 0.0 true)
    (Utilities|FlowControl|Delay (Variables|Default|GetBlend%20Time))
    (bind _newtrack_0 (Timeline|Timeline Play)
      (:Update
        (Transformation|SetRelativeLocation (Variables|Default|GetDoor) (Math|Vector|Lerp(Vector) "0.000000,0.000000,150.000000" "0.000000,0.000000,-130.000000" _newtrack_0) false false))
      (:Finished
        (Utilities|FlowControl|Delay 2.0) ; waiting 2 seconds while the door opens
        (Game|Player|SetViewTargetwithBlend (Game|GetPlayerController 0) NewViewTarget (/ (Variables|Default|GetBlend%20Time) 2.0) "VTBlend_Cubic" 0.0 false) ; shift camera back to player
        (Variables|Default|SetClosed false)))))

(event Custom|QuietOpen
  (bind _newtrack_0 (Timeline|Timeline_0 Play)
    (:Update
      (Transformation|SetRelativeLocation (Variables|Default|GetDoor) (Math|Vector|Lerp(Vector) "0.000000,0.000000,150.000000" "0.000000,0.000000,-130.000000" _newtrack_0) false false))
    (:Finished
      (Variables|Default|SetClosed false))))

(fn ConstructionScript)