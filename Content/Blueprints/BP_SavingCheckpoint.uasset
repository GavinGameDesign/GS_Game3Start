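; Checkpoint actor that records a respawn transform when the third-person player character enters its trigger sphere.
; On overlap it passes GM_Coding2Real's Checkpoint a transform built from a point just above the Cube and the player's rotation and scale.
; It then activates the CheckpointSystem component with a reset.
; An assignment to LastSavedLocation is left unconnected and never runs.
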(event OnComponentBeginOverlap(Sphere)
  (params (OverlappedComponent :type Primitive%20Component%20Object%20Reference) (OtherActor :type Actor%20Object%20Reference) (OtherComp :type Primitive%20Component%20Object%20Reference) (OtherBodyIndex :type Integer) (bFromSweep :type Boolean) (SweepResult :type Hit%20Result%20Structure%20%28by%20ref%29))
  (bind _returnvalue (Transformation|GetActorTransform OtherActor))
  (Utilities|Casting|CastToBP_ThirdPersonCharacter OtherActor)
  (bind _asgm_coding_2real (Utilities|Casting|CastToGM_Coding2Real (Game|GetGameMode)))
  (Default|Checkpoint _asgm_coding_2real (Math|Transform|MakeTransform (+ (Transformation|GetWorldLocation (Variables|Default|GetCube)) "0.000000,0.000000,100.000000") (.rotation _returnvalue) (.scale _returnvalue)))
  (Components|Activation|Activate (Variables|Default|GetCheckpointSystem) true))

(event EventBeginPlay)

(event Collision|EventActorBeginOverlap
  (params (OtherActor :type Actor%20Object%20Reference)))

(event EventTick
  (params (DeltaSeconds :type Float%20%28single-precision%29)))

(fn ConstructionScript)