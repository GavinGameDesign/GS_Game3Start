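; BP_DialogueManager is a proximity-triggered actor that plays a linear dialogue from DT_Dialogue.
; Entering its sphere enables input and shows a press-E prompt, removed on exit.
; The first E press opens the dialogue widget and disables pawn input; every press loads the next row's text, emotion and speaker image.
; When no row is found, it closes the widget, restores pawn input and rearms the DoOnce for replay.
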(event OnComponentBeginOverlap(Sphere)
  (params (OverlappedComponent :type Primitive%20Component%20Object%20Reference) (OtherActor :type Actor%20Object%20Reference) (OtherComp :type Primitive%20Component%20Object%20Reference) (OtherBodyIndex :type Integer) (bFromSweep :type Boolean) (SweepResult :type Hit%20Result%20Structure%20%28by%20ref%29))
  (Utilities|Casting|CastToBP_ThirdPersonCharacter OtherActor)
  (Input|EnableInput (Game|GetPlayerController 0))
  (UserInterface|Viewport|AddtoViewport (Variables|Default|GetPressEWidget) 0))

(event OnComponentEndOverlap(Sphere)
  (params (OverlappedComponent :type Primitive%20Component%20Object%20Reference) (OtherActor :type Actor%20Object%20Reference) (OtherComp :type Primitive%20Component%20Object%20Reference) (OtherBodyIndex :type Integer))
  (Utilities|Casting|CastToBP_ThirdPersonCharacter OtherActor)
  (Input|DisableInput (Game|GetPlayerController 0))
  (Widget|RemovefromParent (Variables|Default|GetPressEWidget)))

(event Custom|Continue
  (bind _dialoguewidget (Variables|Default|GetDialogueWidget))
  (bind _outrownames (DataTable|GetDataTableRowNames "/Game/DataTables/Dialogue/DT_Dialogue.DT_Dialogue"))
  (bind _returnvalue (Utilities|GetDataTableRow "/Game/DataTables/Dialogue/DT_Dialogue.DT_Dialogue" (Utilities|Array|Get(acopy) _outrownames (Variables|Default|GetDialogueIndex)))
    (:then
      (Variables|/Script/UMG.TextBlock|SetText (Variables|/Game/DataTables/Dialogue/W_Dialogue.W_Dialogue_C|GetText _dialoguewidget) (.text _returnvalue))
      (Variables|/Script/UMG.TextBlock|SetText (Variables|/Game/DataTables/Dialogue/W_Dialogue.W_Dialogue_C|GetEmotion _dialoguewidget) (Utilities|Array|Get(acopy) (Variables|Default|GetEmotions) (Math|Conversions|ToInteger(Byte) (.emotion _returnvalue))))
      (Appearance|SetBrushfromTexture (Variables|/Game/DataTables/Dialogue/W_Dialogue.W_Dialogue_C|GetImage_0 _dialoguewidget) (Utilities|Array|Get(acopy) (Variables|Default|GetCharacterImages) (Math|Conversions|ToInteger(Byte) (.speaker _returnvalue))) true)
      (Math|Integer|IncrementInt (Variables|Default|GetDialogueIndex)))
    (:RowNotFound
      (CallFunction|Reset))))

(event Custom|Reset
  (Utilities|FlowControl|Sequence
    (:then_0
      (Variables|Default|SetDialogueIndex 0)
      (Widget|RemovefromParent (Variables|Default|GetDialogueWidget))
      (Input|EnableInput (Game|Player|GetPlayerPawn 0) (Game|GetPlayerController 0)))
    (:then_1
      (Utilities|FlowControl|DoOnce false) ; enters at Reset
    )))

(event EventBeginPlay
  (bind _returnvalue (UserInterface|CreateWidget "/Game/DataTables/Dialogue/W_PressE.W_PressE_C"))
  (Variables|Default|SetPressEWidget _returnvalue)
  (bind _returnvalue_2 (UserInterface|CreateWidget "/Game/DataTables/Dialogue/W_Dialogue.W_Dialogue_C"))
  (Variables|Default|SetDialogueWidget _returnvalue_2))

(event Input|KeyboardEvents|E
  (params (Key :type Key%20Structure :default "None"))
  (:Pressed
    (Utilities|FlowControl|Sequence
      (:then_0
        (Utilities|FlowControl|DoOnce false
          (:Completed
            (Widget|RemovefromParent (Variables|Default|GetPressEWidget))
            (UserInterface|Viewport|AddtoViewport (Variables|Default|GetDialogueWidget) 0)
            (Input|DisableInput (Game|Player|GetPlayerPawn 0) (Game|GetPlayerController 0)))))
      (:then_1
        (CallFunction|Continue)))))

(fn ConstructionScript)