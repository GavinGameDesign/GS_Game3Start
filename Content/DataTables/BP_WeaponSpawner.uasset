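; BP_WeaponSpawner is a pickup-style spawner that creates a random weapon whenever the third-person character overlaps its Sphere1 trigger.
; It picks a random DT_Weapons row and spawns BP_Weapon just above the Sphere component, with no guard against repeat spawns.
; The row's weapon type, elemental type and base damage (as MinDamage) are copied to the weapon before RandomizeValues runs.
; Nodes that set the weapon's text displays are left disconnected.
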(event OnComponentBeginOverlap(Sphere1)
  (params (OverlappedComponent :type Primitive%20Component%20Object%20Reference) (OtherActor :type Actor%20Object%20Reference) (OtherComp :type Primitive%20Component%20Object%20Reference) (OtherBodyIndex :type Integer) (bFromSweep :type Boolean) (SweepResult :type Hit%20Result%20Structure%20%28by%20ref%29))
  (Utilities|Casting|CastToBP_ThirdPersonCharacter OtherActor)
  (CallFunction|SpawnWeapon))

(event Custom|SpawnWeapon
  (bind _sphere (Variables|Default|GetSphere))
  (bind _returnvalue (Transformation|GetWorldLocation _sphere))
  (bind _outrownames (DataTable|GetDataTableRowNames "/Game/DataTables/DT_Weapons.DT_Weapons"))
  (bind _returnvalue_2 (Utilities|GetDataTableRow "/Game/DataTables/DT_Weapons.DT_Weapons" (.OutItem (Utilities|Array|Random _outrownames)))
    (:then
      (bind _returnvalue_3 (Game|SpawnActorfromClass "/Game/DataTables/BP_Weapon.BP_Weapon_C" (Math|Transform|MakeTransform (Math|Vector|MakeVector (.x _returnvalue) (.y _returnvalue) (+ (.z _returnvalue) 2e+01)) "0, 0, 0" "1.000000,1.000000,1.000000") "Undefined" "MultiplyWithRoot" 0 0))
      (Variables|/Game/DataTables/BP_Weapon.BP_Weapon_C|SetWeaponType _returnvalue_3 (.weapontype _returnvalue_2))
      (Variables|/Game/DataTables/BP_Weapon.BP_Weapon_C|SetElementalType _returnvalue_3 (.elementaltype _returnvalue_2))
      (Variables|/Game/DataTables/BP_Weapon.BP_Weapon_C|SetMinDamage _returnvalue_3 (.basedamage _returnvalue_2))
      (Default|RandomizeValues _returnvalue_3))))

(fn ConstructionScript)